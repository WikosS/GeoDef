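; BPC_BulletShooter is a component that fires bullets as Niagara particle systems and damages enemies they touch.
; SpawnBullet spawns a colored NS_Bullet2 with itself as callback, while SpawnPatternBullet and ShotSpread repeat it over a transform array or stepped yaw angles.
; Exported particle positions return through ParticleData, which sphere-overlaps each for BP_Enemies and applies fixed damage, ignoring the Damage passed to the spawn functions.
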(event `self.ReceiveParticleData`
  (params (Data :type "Array of BasicParticleData Structure (by ref)") (NiagaraSystem :type "NiagaraSystem Object Reference") (SimulationPositionOffset :type "Vector Structure (by ref)"))
  (for _array_element Data
    (bind _outactors (`KismetSystemLibrary.SphereOverlapActors` (`.Position` (break `BasicParticleData` _array_element)) 20.0 (`|MakeArray` "ObjectTypeQuery2" "ObjectTypeQuery1" :!type "EObjectTypeQuery Enum") "/Game/Blueprint/Enemies/BP_Enemies.BP_Enemies_C"))
    (for _array_element_2 _outactors
      (`GameplayStatics.ApplyDamage` _array_element_2 1.0))))

(fn `ShotSpread`
  (params (Damage :type "Float (double-precision)") (Color :type "Color Structure") (Transform :type "Transform Structure") (BulletNb :type Integer))
  (locals (SpreadAngle :type "Float (double-precision)" :default 10.0))
  (for _index (range 1 (+ BulletNb 1))
    (`self.Spawn Bullet` Color Damage (`KismetMathLibrary.MakeTransform` (.location Transform) (`KismetMathLibrary.MakeRotator` (.roll (.rotation Transform)) (.pitch (.rotation Transform)) (+ (.yaw (.rotation Transform)) (* _index (`local.SpreadAngle`))))))))

(fn `Spawn Bullet`
  (params (Color :type "Color Structure") (Damage :type "Float (double-precision)") (Transform :type "Transform Structure"))
  (bind _returnvalue (`NiagaraFunctionLibrary.SpawnSystemAtLocation` "/Game/Niagara/Bullet_two/NS_Bullet2.NS_Bullet2" Transform_Location Transform_Rotation (1.0 1.0 1.0) true true "ManualRelease"))
  (`FXSystemComponent.SetColorParameter` _returnvalue "ParticleColor" (`KismetMathLibrary.Conv_ColorToLinearColor` Color))
  (`NiagaraComponent.SetVariableObject` _returnvalue "BPCallback" self))

(fn `SpawnPatternBullet`
  (params (Color :type "Color Structure") (Damage :type "Float (double-precision)") (Pattern :type "Array of Transform Structure"))
  ;[1 1 1] Pattern is an array of transform
  (for _array_element Pattern
    (`self.Spawn Bullet` Color Damage _array_element)))