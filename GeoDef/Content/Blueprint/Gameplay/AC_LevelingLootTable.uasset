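; Component that holds a leveling loot table and picks a random entry from it by weight.
; ChooseLoot rolls between zero and the sum of all LootTable values from CalculateSum, then returns the first key whose running weight reaches the roll.
; GetStats looks up the value stored in StatsTable for a given name.
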(fn `CalculateSum`
  (returns (Total :type "Float (double-precision)"))
  (locals (Totals :type "Float (double-precision)"))
  (bind _totals (`local.Totals`))
  (bind _values (`BlueprintMapLibrary.Map_Values` (`self.LootTable`)))
  (for _array_element _values
    (set `local.Totals` (+ _array_element _totals)))
  (return _totals))

(fn `ChooseLoot`
  (returns (Name :type Name))
  (locals (Sums :type "Float (double-precision)") (Rolled :type "Float (double-precision)" :default 0.0) (Weight :type "Float (double-precision)"))
  (bind _total (`self.CalculateSum`))
  (set `local.Sums` _total)
  (set `local.Rolled` (`KismetMathLibrary.RandomFloatInRange` 0.0 (`local.Sums`)))
  (bind _keys (`BlueprintMapLibrary.Map_Keys` (`self.LootTable`)))
  (for _array_element _keys
    (bind _output_get (set `local.Weight` (+ (`BlueprintMapLibrary.Map_Find` (`self.LootTable`) _array_element) (`local.Weight`))))
    (if (>= _output_get (`local.Rolled`))
      (return _array_element))))

(fn `GetStats`
  (params (Name :type Name))
  (returns (Stats :type "/Game/Blueprint/Gameplay/S_Stats Structure"))
  (return (`BlueprintMapLibrary.Map_Find` (`self.StatsTable`) Name)))