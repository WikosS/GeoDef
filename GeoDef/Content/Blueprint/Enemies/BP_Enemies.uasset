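; BP_Enemies is an enemy actor that deals periodic melee-range damage to the player character and awards XP when killed.
; A looping timer started on BeginPlay calls Attack, which damages every BP_ThirdPersonCharacter overlapping the AttackCollision volume.
; Incoming damage reduces Health; at zero, XpDrop goes to the damage causer and the enemy is destroyed, but only if that causer casts to BP_ThirdPersonCharacter.
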(event `self.ReceiveBeginPlay`
  (`KismetSystemLibrary.K2_SetTimer` null "Attack" 2.0 true))

(event `self.ReceiveAnyDamage`
  (params (Damage :type "Float (single-precision)") (DamageType :type "DamageType Object Reference") (InstigatedBy :type "Controller Object Reference") (DamageCauser :type "Actor Object Reference"))
  (set `self.Health` (- (`self.Health`) Damage))
  (if (<= (`self.Health`) 0.0)
    (bind _asbp_third_person_character (cast `/Game/ThirdPerson/Blueprints/BP_ThirdPersonCharacter` DamageCauser))
    (`/Game/ThirdPerson/Blueprints/BP_ThirdPersonCharacter.EarnXP` _asbp_third_person_character (`self.XpDrop`))
    (`self.K2_DestroyActor`)))

(fn `Attack`
  (for _array_element (`PrimitiveComponent.GetOverlappingActors` (`self.AttackCollision`) "/Game/ThirdPerson/Blueprints/BP_ThirdPersonCharacter.BP_ThirdPersonCharacter_C")
    (`GameplayStatics.ApplyDamage` _array_element (`self.Damage`) null self "/Script/Engine.DamageType")))

(fn `UserConstructionScript`)