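; BP_EnemiesSpawner is an endless enemy spawner that escalates difficulty as its spawn count grows.
; Tick accumulates delta time and spawns BP_Enemies at random SpawnLoc transforms each time SpawnDelay elapses, catching up through a loop.
; Each successful spawn receives current Damage and Health, then increments Spawned and recalculates stats.
; Exponential curves on integer-divided spawn counts shorten the delay and raise health and damage in steps.
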(event `self.ReceiveBeginPlay`
  (set `self.SpawnDelay` (`self.BaseSpawnInterval`))
  (set `self.Damage` (`self.BaseDamage`))
  (set `self.Health` (`self.BaseHP`)))

(event `self.ReceiveTick`
  (params (DeltaSeconds :type "Float (single-precision)"))
  (bind _spawnloc (`self.SpawnLoc`))
  ;[1 1 1] Add delta to the stack
  (set `self.DeltaStack` (+ DeltaSeconds (`self.DeltaStack`)))
  ;[1 1 1] Remove the spawn delay from the stack
  (while (>= (`self.DeltaStack`) (`self.SpawnDelay`))
    (set `self.DeltaStack` (- (`self.DeltaStack`) (`self.SpawnDelay`)))
    ;[1 1 1] SpawnActor
    (bind _returnvalue (`|SpawnActorFromClass` "/Game/Blueprint/Enemies/BP_Enemies.BP_Enemies_C" (`|GetArrayItem` _spawnloc (`KismetMathLibrary.RandomInteger` (`KismetArrayLibrary.Array_Length` _spawnloc))) "Undefined" "MultiplyWithRoot" null null))
    (if (`KismetSystemLibrary.IsValid` _returnvalue)
      ;[1 1 1] Set Spawned Actor stats
      (set `/Game/Blueprint/Enemies/BP_Enemies.Damage` (`self.Damage`) _returnvalue)
      (set `/Game/Blueprint/Enemies/BP_Enemies.Health` (`self.Health`) _returnvalue)
      ;[1 1 1] Increase spawned count
      (set `self.Spawned` (+ (`self.Spawned`) 1))
      (`self.Recalc_Stats`)
      (else
        (`KismetSystemLibrary.PrintString` "Failed to spawn Enemies")))))

(event `Recalc_Stats`
  (bind _spawned (`self.Spawned`))
  (bind _returnvalue (`KismetMathLibrary.Conv_IntToDouble` (/ _spawned 9)))
  (set `self.SpawnDelay` (* (`self.BaseSpawnInterval`) (`KismetMathLibrary.MultiplyMultiply_FloatFloat` 0.95 _returnvalue)))
  (set `self.Health` (* (`self.BaseHP`) (`KismetMathLibrary.MultiplyMultiply_FloatFloat` 1.45 (`KismetMathLibrary.Conv_IntToDouble` (/ _spawned 5)))))
  (set `self.Damage` (* (`self.BaseDamage`) (`KismetMathLibrary.MultiplyMultiply_FloatFloat` 1.2 _returnvalue))))

(fn `UserConstructionScript`)